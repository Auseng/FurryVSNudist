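; Player character Blueprint that handles health, suit loss on damage and game over, plus Escape to quit.
; BeginPlay creates a hidden health bar widget.
; Damage at 50 health or below swaps the player's mesh to Ulv and sets jump and walk speed.
; At zero it shows a game-over widget, then destroys itself before the delayed "Park" level reload; a death montage is left unwired.
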(event EventBeginPlay
  ;[1 1 1] HealthBar
  (bind _returnvalue (UserInterface|CreateWidget "/Game/HUD/HealthBar.HealthBar_C"))
  (bind _output_get (Variables|Default|SetHealthBar%20Reference _returnvalue))
  (UserInterface|Viewport|AddtoViewport _output_get 0)
  (Widget|SetVisibility _output_get "Hidden"))

(event Game|Damage|EventAnyDamage
  (params (Damage :type Float%20%28single-precision%29) (DamageType :type Damage%20Type%20Object%20Reference) (InstigatedBy :type Controller%20Object%20Reference) (DamageCauser :type Actor%20Object%20Reference))
  (bind _returnvalue (Game|GetPlayerCharacter 0))
  (bind _charactermovement (Variables|/Script/Engine.Character|GetCharacterMovement _returnvalue))
  ;[1 1 1] Loss of suit on damage, Game Over and Restart
  (bind _output_get (Variables|Default|SetCurrentHealth (- (Variables|Default|GetCurrentHealth) Damage)))
  (if (<= _output_get 5e+01)
    (Class|SkinnedMeshComponent|SetSkeletalMesh (Variables|/Script/Engine.Character|GetMesh _returnvalue) "/Game/Meshes/Characters/Ulv.Ulv" true)
    (Variables|/Script/Engine.CharacterMovementComponent|SetJumpZVelocity _charactermovement 4e+02)
    (Variables|/Script/Engine.CharacterMovementComponent|SetMaxWalkSpeed _charactermovement 5e+02)
    (if (<= _output_get 0.0)
      (bind _returnvalue_2 (UserInterface|CreateWidget "/Game/HUD/GameOver.GameOver_C"))
      (bind _output_get_2 (Variables|Default|SetGameOver _returnvalue_2))
      (UserInterface|Viewport|AddtoViewport _output_get_2 0)
      (Utilities|FlowControl|Delay 1.0)
      (Actor|DestroyActor)
      (Utilities|FlowControl|Delay 2.0)
      (Game|OpenLevel(byName) "Park"))))

(event Input|KeyboardEvents|Escape
  (params (Key :type Key%20Structure))
  (:Pressed
    (Game|QuitGame 0 "Quit")
    (Development|ExecuteConsoleCommand "Exit")))

(fn ConstructionScript)