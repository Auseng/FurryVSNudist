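; Cheetah Suit pickup that changes the player's look when touched by an FCharacter_BP.
; On overlap it destroys its mesh and collision, swaps player 0's skeletal mesh to Gepard and plays a sound, leaving the actor alive.
; While idle it rotates every Tick and moves by Timeline-driven offsets, both frame-based.
; Walk speed, jump velocity and DestroyActor nodes exist but are unconnected, so the suit grants no stat change.
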(event Collision|EventActorBeginOverlap
  (params (OtherActor :type Actor%20Object%20Reference))
  ;[1 1 1] Bunny Suit
  (Utilities|Casting|CastToFCharacter_BP OtherActor)
  (Components|DestroyComponent (Variables|Default|GetStaticMesh))
  (Components|DestroyComponent (Variables|Default|GetCollision))
  (Development|PrintString "Put on Cheetah Suit")
  (Class|SkinnedMeshComponent|SetSkeletalMesh (Variables|/Script/Engine.Character|GetMesh (Game|GetPlayerCharacter 0)) "/Game/Meshes/Costumes/Gepard.Gepard" true)
  (Audio|PlaySound2D "/Game/Audio/PlayerProjectileWallHit16-bit.PlayerProjectileWallHit16-bit"))

(event EventTick
  (params (DeltaSeconds :type Float%20%28single-precision%29))
  ;[1 1 1] Power up idle
  (Transformation|AddActorLocalRotation "0,1.000000, 0" false false)
  (bind _movement (Timeline|Timeline_0 Play)
    (:Update
      (Transformation|AddActorLocalOffset _movement false false))))

(fn ConstructionScript)