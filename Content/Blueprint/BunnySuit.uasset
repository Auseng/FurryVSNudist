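; BunnySuit is a power-up pickup that dresses the player in a bunny suit when a character overlaps it.
; On overlap with an FCharacter_BP it removes its mesh and collision, swaps player 0's skeletal mesh to Kanin, sets new jump velocity and walk speed, then destroys itself.
; While idle, Tick spins it and plays a Movement timeline that offsets its local position.
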(event Collision|EventActorBeginOverlap
  (params (OtherActor :type Actor%20Object%20Reference))
  (bind _returnvalue (Game|GetPlayerCharacter 0))
  (bind _charactermovement (Variables|/Script/Engine.Character|GetCharacterMovement _returnvalue))
  ;[1 1 1] Bunny Suit
  (Utilities|Casting|CastToFCharacter_BP OtherActor)
  (Components|DestroyComponent (Variables|Default|GetStaticMesh))
  (Components|DestroyComponent (Variables|Default|GetCollision))
  (Development|PrintString "Put on Bunny Suit")
  (Class|SkinnedMeshComponent|SetSkeletalMesh (Variables|/Script/Engine.Character|GetMesh _returnvalue) "/Game/Meshes/Costumes/Kanin.Kanin" true)
  (Variables|/Script/Engine.CharacterMovementComponent|SetJumpZVelocity _charactermovement 7e+02)
  (Variables|/Script/Engine.CharacterMovementComponent|SetMaxWalkSpeed _charactermovement 5e+02)
  (Actor|DestroyActor))

(event EventTick
  (params (DeltaSeconds :type Float%20%28single-precision%29))
  ;[1 1 1] Power up idle
  (Transformation|AddActorLocalRotation "0,1.000000, 0" false false)
  (bind _movement (Timeline|Movement Play)
    (:Update
      (Transformation|AddActorLocalOffset _movement false false))))

(fn ConstructionScript)