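; Boss AI character that runs one of four behaviours by AIState: roam, chase player, nudist idle or patrol between two target points.
; Behaviours are self-repeating AIMoveTo loops; seeing the player triggers a chase that jumps and deals damage on reaching them.
; Player death disables pawn sensing, which gates the chase, and re-runs the state selection.
; Projectile overlaps decrement HitCounter; at zero the boss swaps mesh, is destroyed and shows the Winner widget.
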(event OnSeePawn(PawnSensing)
  (params (Pawn :type Pawn%20Object%20Reference))
  ;[1 1 1] Chase on sight
  (bind _asfcharacter_bp (Utilities|Casting|CastToFCharacter_BP Pawn))
  (Variables|Default|SetChase? true)
  (CallFunction|ChasePlayer _asfcharacter_bp))

(event Custom|Nudist%20Idle
  ;[1 1 1] Nudist Idle State
  (AI|AIMoveTo self (.RandomLocation (Class|NavigationSystem|GetRandomPointinNavigableRadius (Transformation|GetActorLocation) 1e+01)) 0 5.0 false
    (:OnSuccess
      (Utilities|FlowControl|Delay 2.0)
      (CallFunction|NudistIdle))))

(event Custom|ChasePlayer
  (params (PlayerToChase :type Pawn%20Object%20Reference))
  ;[1 1 1] Chase Player State
  (Variables|Default|SetChase? true)
  (if (Variables|/Script/AIModule.PawnSensingComponent|GetbEnableSensingUpdates (Variables|Default|GetPawnSensing))
    (AI|AIMoveTo self "0, 0, 0" PlayerToChase 0.0 false
      (:OnSuccess
        (Character|Jump)
        (Game|Damage|ApplyDamage PlayerToChase (Variables|Default|GetDamage) 0 PlayerToChase)
        (Utilities|FlowControl|Delay 2.0)
        (CallFunction|ChasePlayer PlayerToChase)))))

(event Custom|Roam
  ;[1 1 1] Roam State
  (if (Variables|Default|GetChase?)
    (CallFunction|ChasePlayer (Game|GetPlayerCharacter 0))
    (else
      (AI|AIMoveTo self (.RandomLocation (Class|NavigationSystem|GetRandomPointinNavigableRadius (Transformation|GetActorLocation) 1e+02)) 0 5.0 false
        (:OnSuccess
          (Utilities|FlowControl|Delay 2.0)
          (CallFunction|Roam))))))

(event Custom|Patrol
  ;[1 1 1] Patrol State
  (AI|AIMoveTo self "0, 0, 0" (Variables|Default|GetTargetPoint1) 5.0 false
    (:OnSuccess
      (Utilities|FlowControl|Delay 5.0)
      (AI|AIMoveTo self "0, 0, 0" (Variables|Default|GetTargetPoint2) 5.0 false
        (:OnSuccess
          (Utilities|FlowControl|Delay 5.0)
          (CallFunction|Patrol))))))

(event Custom|ResetAI
  ;[1 1 1] Initial AI Selection and Reset
  (Class|PawnSensingComponent|SetSensingUpdatesEnabled (Variables|Default|GetPawnSensing) false)
  (switch Utilities|FlowControl|Switch|SwitchonE_AIState (Variables|Default|GetAIState)
    (:NewEnumerator1
      (CallFunction|Roam))
    (:NewEnumerator2
      (CallFunction|ChasePlayer))
    (:NewEnumerator4
      (CallFunction|NudistIdle))
    (:NewEnumerator3
      (CallFunction|Patrol))))

(event EventBeginPlay
  ;[1 1 1] Initial AI Selection and Reset
  (bind _asfcharacter_bp (Utilities|Casting|CastToFCharacter_BP (Game|GetPlayerCharacter 0)))
  (EventDispatchers|BindEventtoPlayerDied _asfcharacter_bp (delegate Custom|ResetAI))
  ;[1 1 1] AI Selection
  (switch Utilities|FlowControl|Switch|SwitchonE_AIState (Variables|Default|GetAIState)
    (:NewEnumerator1
      (CallFunction|Roam))
    (:NewEnumerator2
      (CallFunction|ChasePlayer))
    (:NewEnumerator4
      (CallFunction|NudistIdle))
    (:NewEnumerator3
      (CallFunction|Patrol))))

(event Collision|EventActorBeginOverlap
  (params (OtherActor :type Actor%20Object%20Reference))
  ;[1 1 1] Destroy on hit
  (Utilities|Casting|CastToMyFProjectile OtherActor)
  (bind _output_get (Variables|Default|SetHitCounter (- (Variables|Default|GetHitCounter) 1.0)))
  (if (<= _output_get 0.0)
    (Class|SkinnedMeshComponent|SetSkeletalMesh (Variables|Character|GetMesh) "/Game/Meshes/Characters/Nudistledermedt-skjorte.Nudistledermedt-skjorte" true)
    (Utilities|FlowControl|Delay 2.0)
    (Actor|DestroyActor)
    (bind _returnvalue (UserInterface|CreateWidget "/Game/HUD/Winner.Winner_C"))
    (bind _output_get_2 (Variables|Default|SetWinner _returnvalue))
    (UserInterface|Viewport|AddtoViewport _output_get_2 0)))

(fn ConstructionScript)